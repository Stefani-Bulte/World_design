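; A standing light prop Blueprint whose colour is chosen through a Colour key.
; The Construction Script looks that key up in two maps, tinting the PointLight from LightColours and a glow material from MaterialColours.
; It creates a dynamic instance of Glow_Mat, sets its EmissiveColour parameter and applies it to the StandingLight mesh's fourth material slot.
; The event graph holds no active logic.
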(event EventBeginPlay)

(event Collision|EventActorBeginOverlap
  (params (OtherActor :type Actor%20Object%20Reference)))

(event EventTick
  (params (DeltaSeconds :type Float%20%28single-precision%29)))

(fn ConstructionScript
  (Rendering|Components|Light|SetLightColor (Variables|Default|GetPointLight) (.Value (Utilities|Map|Find (Variables|Default|GetLightColours) (Variables|Default|GetColour))) true)
  (bind _returnvalue (Rendering|Material|CreateDynamicMaterialInstance "/Game/Meshes/Glow_Mat.Glow_Mat" :!class /Script/Engine.KismetMaterialLibrary))
  (bind _output_get (Variables|Default|SetLightMaterial _returnvalue))
  (Rendering|Material|SetVectorParameterValue _output_get "EmissiveColour" (.Value (Utilities|Map|Find (Variables|Default|GetMaterialColours) (Variables|Default|GetColour))) :!class /Script/Engine.MaterialInstanceDynamic)
  (Rendering|Material|SetMaterial (Variables|Default|Getstanding_light) 3 (Variables|Default|GetLightMaterial)))